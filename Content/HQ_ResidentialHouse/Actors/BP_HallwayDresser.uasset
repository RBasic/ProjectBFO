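; BP_HallwayDresser is a hallway dresser prop with three drawers that toggle open and closed individually.
; The OpenDoor event compares the hit component to each drawer mesh and flips that drawer's open flag.
; Each drawer has its own timeline, played to open and reversed to close, that drives its relative Y location while keeping X and Z.
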(event EventOpenDoor
  (params (hitComponent :type Actor%20Component%20Object%20Reference))
  (bind _hallwaydresser_drawer_c (Variables|Default|GetHallwayDresser_Drawer_C))
  (bind _hallwaydresser_drawer_a (Variables|Default|GetHallwayDresser_Drawer_A))
  (bind _hallwaydresser_drawer_b (Variables|Default|GetHallwayDresser_Drawer_B))
  (bind _relativelocation (Variables|/Script/Engine.SceneComponent|GetRelativeLocation _hallwaydresser_drawer_c))
  (bind _relativelocation_2 (Variables|/Script/Engine.SceneComponent|GetRelativeLocation _hallwaydresser_drawer_a))
  (bind _relativelocation_3 (Variables|/Script/Engine.SceneComponent|GetRelativeLocation _hallwaydresser_drawer_b))
  (if (== hitComponent (Variables|Default|GetHallwayDresser_Drawer_A))
    (if (not (Variables|Default|GetOpenDrawerA?))
      (Variables|Default|SetOpenDrawerA? true)
      (bind _movement (Timeline|Timeline_0 Play)
        (:Update
          (Transformation|SetRelativeLocation _hallwaydresser_drawer_a (Math|Vector|MakeVector (.x _relativelocation_2) _movement (.z _relativelocation_2)) false false)))
      (else
        (Variables|Default|SetOpenDrawerA? false)
        (Timeline|Timeline_0 Reverse)))
    (elif (== hitComponent (Variables|Default|GetHallwayDresser_Drawer_B))
      (if (not (Variables|Default|GetOpenDrawerB?))
        (Variables|Default|SetOpenDrawerB? true)
        (bind _movement_2 (Timeline|Timeline_1 Play)
          (:Update
            (Transformation|SetRelativeLocation _hallwaydresser_drawer_b (Math|Vector|MakeVector (.x _relativelocation_3) _movement_2 (.z _relativelocation_3)) false false)))
        (else
          (Variables|Default|SetOpenDrawerB? false)
          (Timeline|Timeline_1 Reverse)))
      (elif (== hitComponent (Variables|Default|GetHallwayDresser_Drawer_C))
        (if (not (Variables|Default|GetOpenDrawerC?))
          (Variables|Default|SetOpenDrawerC? true)
          (bind _movement_3 (Timeline|Timeline_2 Play)
            (:Update
              (Transformation|SetRelativeLocation _hallwaydresser_drawer_c (Math|Vector|MakeVector (.x _relativelocation) _movement_3 (.z _relativelocation)) false false)))
          (else
            (Variables|Default|SetOpenDrawerC? false)
            (Timeline|Timeline_2 Reverse)))))))

(fn ConstructionScript)
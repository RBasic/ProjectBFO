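; BP_ToiletTable is a toilet table prop for the residential house with a drawer that toggles open and closed.
; Each OpenDoor event flips a boolean, posts a Wwise drawer sound, and plays or reverses a timeline.
; The timeline's Movement track drives the drawer component's relative Y location, keeping X and Z unchanged.
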(event EventOpenDoor
  (params (hitComponent :type Actor%20Component%20Object%20Reference))
  (bind _self self)
  (bind _toilettable_drawer (Variables|Default|GetToiletTable_Drawer))
  (bind _relativelocation (Variables|/Script/Engine.SceneComponent|GetRelativeLocation _toilettable_drawer))
  (if (not (Variables|Default|GetOpenDrawerA?))
    (Variables|Default|SetOpenDrawerA? true)
    (Class|AkGameplayStatics|PostEvent "/Game/WwiseAudio/Events/Hassan/Play_SC_Drawner.Play_SC_Drawner" _self)
    (bind _movement (Timeline|Timeline_0 Play)
      (:Update
        (Transformation|SetRelativeLocation _toilettable_drawer (Math|Vector|MakeVector (.x _relativelocation) _movement (.z _relativelocation)) false false)))
    (else
      (Variables|Default|SetOpenDrawerA? false)
      (Class|AkGameplayStatics|PostEvent "/Game/WwiseAudio/Events/Hassan/Play_SC_Drawner.Play_SC_Drawner" _self)
      (Timeline|Timeline_0 Reverse))))

(fn ConstructionScript)
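; BP_Cabinet is a cabinet actor with left and right doors that toggle open and closed.
; The OpenDoor event flips an Open flag and plays or reverses a timeline.
; The timeline's Angle track sets the relative yaw of both doors, negated on the right one so they swing in opposite directions.
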(event EventOpenDoor
  (params (hitComponent :type Actor%20Component%20Object%20Reference))
  (if (not (Variables|Default|GetOpen?))
    (Variables|Default|SetOpen? true)
    (bind _angle (Timeline|Timeline_0 Play)
      (:Update
        (Transformation|SetRelativeRotation (Variables|Default|GetCabinet_Door_L) (Math|Rotator|MakeRotator 0.0 0.0 _angle) false false)
        (Transformation|SetRelativeRotation (Variables|Default|GetCabinet_Door_R) (Math|Rotator|MakeRotator 0.0 0.0 (* _angle -1.0)) false false)))
    (else
      (Variables|Default|SetOpen? false)
      (Timeline|Timeline_0 Reverse))))

(fn ConstructionScript)
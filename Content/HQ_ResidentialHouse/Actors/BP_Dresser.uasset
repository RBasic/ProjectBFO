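; BP_Dresser is an interactive dresser prop for the residential house set, with three drawers that open and close independently.
; Its OpenDoor event matches the hit component to a drawer, flips that drawer's open flag and posts a Wwise drawer sound.
; Each drawer has its own timeline, played or reversed to slide it along its relative Y axis.
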(event EventBeginPlay)

(event Collision|EventActorBeginOverlap
  (params (OtherActor :type Actor%20Object%20Reference)))

(event EventTick
  (params (DeltaSeconds :type Float%20%28single-precision%29)))

(event EventOpenDoor
  (params (hitComponent :type Actor%20Component%20Object%20Reference))
  (bind _self self)
  (bind _dresser_drawerb (Variables|Default|GetDresser_DrawerB))
  (bind _dresser_drawerc (Variables|Default|GetDresser_DrawerC))
  (bind _dresser_drawera (Variables|Default|GetDresser_DrawerA))
  (bind _relativelocation (Variables|/Script/Engine.SceneComponent|GetRelativeLocation _dresser_drawerc))
  (bind _relativelocation_2 (Variables|/Script/Engine.SceneComponent|GetRelativeLocation _dresser_drawera))
  (bind _relativelocation_3 (Variables|/Script/Engine.SceneComponent|GetRelativeLocation _dresser_drawerb))
  (if (== hitComponent (Variables|Default|GetDresser_DrawerA))
    (if (not (Variables|Default|GetOpenDrawerA?))
      (Variables|Default|SetOpenDrawerA? true)
      (Class|AkGameplayStatics|PostEvent "/Game/WwiseAudio/Events/Hassan/Play_SC_Drawner.Play_SC_Drawner" _self)
      (bind _movement (Timeline|Timeline_2 Play)
        (:Update
          (Transformation|SetRelativeLocation _dresser_drawera (Math|Vector|MakeVector (.x _relativelocation_2) _movement (.z _relativelocation_2)) false false)))
      (else
        (Variables|Default|SetOpenDrawerA? false)
        (Class|AkGameplayStatics|PostEvent "/Game/WwiseAudio/Events/Hassan/Play_SC_Drawner.Play_SC_Drawner" _self)
        (Timeline|Timeline_2 Reverse)))
    (elif (== hitComponent (Variables|Default|GetDresser_DrawerB))
      (if (not (Variables|Default|GetOpenDrawerB?))
        (Variables|Default|SetOpenDrawerB? true)
        (Class|AkGameplayStatics|PostEvent "/Game/WwiseAudio/Events/Hassan/Play_SC_Drawner.Play_SC_Drawner" _self)
        (bind _movement_2 (Timeline|Timeline_0 Play)
          (:Update
            (Transformation|SetRelativeLocation _dresser_drawerb (Math|Vector|MakeVector (.x _relativelocation_3) _movement_2 (.z _relativelocation_3)) false false)))
        (else
          (Variables|Default|SetOpenDrawerB? false)
          (Class|AkGameplayStatics|PostEvent "/Game/WwiseAudio/Events/Hassan/Play_SC_Drawner.Play_SC_Drawner" _self)
          (Timeline|Timeline_0 Reverse)))
      (elif (== hitComponent (Variables|Default|GetDresser_DrawerC))
        (if (not (Variables|Default|GetOpenDrawerC?))
          (Variables|Default|SetOpenDrawerC? true)
          (Class|AkGameplayStatics|PostEvent "/Game/WwiseAudio/Events/Hassan/Play_SC_Drawner.Play_SC_Drawner" _self)
          (bind _movement_3 (Timeline|Timeline_1 Play)
            (:Update
              (Transformation|SetRelativeLocation _dresser_drawerc (Math|Vector|MakeVector (.x _relativelocation) _movement_3 (.z _relativelocation)) false false)))
          (else
            (Variables|Default|SetOpenDrawerC? false)
            (Class|AkGameplayStatics|PostEvent "/Game/WwiseAudio/Events/Hassan/Play_SC_Drawner.Play_SC_Drawner" _self)
            (Timeline|Timeline_1 Reverse)))))))

(fn ConstructionScript)
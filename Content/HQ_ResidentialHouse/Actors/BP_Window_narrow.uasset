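; Narrow house window actor that acts as the Thief's win point.
; Its EndGameThief event casts the passed actor to BP_Thief, sets that thief's message to "Ouvrir" and checks its taken-object count against a hardcoded threshold.
; When enough objects are taken, it creates the HUD_EndGame widget with a Thief victory text, adds it to the viewport and shows the mouse cursor for player controller 0.
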(event Custom|EndGameThief
  (params (Actor :type Actor%20Object%20Reference))
  (bind _asbp_thief (Utilities|Casting|CastToBP_Thief Actor))
  (Variables|/Game/Blueprints/FirstPersonCharacter.FirstPersonCharacter_C|SetMessage _asbp_thief "Ouvrir")
  (if (>= (Variables|/Game/Blueprints/BP_Thief.BP_Thief_C|GetTakenObject _asbp_thief) 5)
    (bind _returnvalue (UserInterface|CreateWidget "/Game/HUD/HUD_EndGame.HUD_EndGame_C"))
    (Rendering|Components|TextRender|SetText (Variables|/Game/HUD/HUD_EndGame.HUD_EndGame_C|GetTextBlock_106 _returnvalue) "The Thief win the game !")
    (Variables|/Script/Engine.PlayerController|SetbShowMouseCursor (Game|GetPlayerController 0) true)
    (UserInterface|Viewport|AddtoViewport _returnvalue 0)))

(fn ConstructionScript)
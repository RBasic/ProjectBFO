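; Interactive kitchen cabinet actor with a hinged door and a sliding drawer that open and close in the game.
; An OpenDoor event checks the hit component: the door mesh toggles the door, and any other component toggles the drawer.
; Each part has its own state flag and a timeline played forward or reversed, driving door yaw or drawer Y position.
; Every toggle posts the same Wwise open/close sound.
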(event EventBeginPlay)

(event Collision|EventActorBeginOverlap
  (params (OtherActor :type Actor%20Object%20Reference)))

(event EventTick
  (params (DeltaSeconds :type Float%20%28single-precision%29)))

(event EventOpenDoor
  (params (hitComponent :type Actor%20Component%20Object%20Reference))
  (bind _self self)
  (bind _kitchensetc_drawer (Variables|Default|GetKitchenSetC_Drawer))
  (bind _relativelocation (Variables|/Script/Engine.SceneComponent|GetRelativeLocation _kitchensetc_drawer))
  (if (== hitComponent (Variables|Default|GetKitchenSetC_Door))
    (if (not (Variables|Default|GetOpenDoor?))
      (Variables|Default|SetOpenDoor? true)
      (Class|AkGameplayStatics|PostEvent "/Game/WwiseAudio/Events/Hassan/Play_SC_Door_Open_Close.Play_SC_Door_Open_Close" _self)
      (bind _angle (Timeline|Timeline_0 Play)
        (:Update
          (Transformation|SetRelativeRotation (Variables|Default|GetKitchenSetC_Door) (Math|Rotator|MakeRotator 0.0 0.0 (* _angle -1.0)) false false)))
      (else
        (Variables|Default|SetOpenDoor? false)
        (Class|AkGameplayStatics|PostEvent "/Game/WwiseAudio/Events/Hassan/Play_SC_Door_Open_Close.Play_SC_Door_Open_Close" _self)
        (Timeline|Timeline_0 Reverse)))
    (elif (not (Variables|Default|GetOpenDrawer?))
      (Variables|Default|SetOpenDrawer? true)
      (Class|AkGameplayStatics|PostEvent "/Game/WwiseAudio/Events/Hassan/Play_SC_Door_Open_Close.Play_SC_Door_Open_Close" _self)
      (bind _movement (Timeline|Timeline_1 Play)
        (:Update
          (Transformation|SetRelativeLocation _kitchensetc_drawer (Math|Vector|MakeVector (.x _relativelocation) _movement (.z _relativelocation)) false false)))
      (else
        (Variables|Default|SetOpenDrawer? false)
        (Class|AkGameplayStatics|PostEvent "/Game/WwiseAudio/Events/Hassan/Play_SC_Door_Open_Close.Play_SC_Door_Open_Close" _self)
        (Timeline|Timeline_1 Reverse)))))

(fn ConstructionScript)
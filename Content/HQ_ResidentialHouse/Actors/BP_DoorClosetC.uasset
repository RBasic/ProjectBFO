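; Closet door actor for the residential house set that swings open or shut each time its OpenDoor event is called.
; An Open flag picks whether the timeline plays forward or reverses, and its Angle track drives the door component's relative yaw.
; Both directions post the same Wwise open/close sound on the actor.
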(event EventBeginPlay)

(event Collision|EventActorBeginOverlap
  (params (OtherActor :type Actor%20Object%20Reference)))

(event EventTick
  (params (DeltaSeconds :type Float%20%28single-precision%29)))

(event EventOpenDoor
  (params (hitComponent :type Actor%20Component%20Object%20Reference))
  (bind _self self)
  (if (not (Variables|Default|GetOpen?))
    (Variables|Default|SetOpen? true)
    (Class|AkGameplayStatics|PostEvent "/Game/WwiseAudio/Events/Hassan/Play_SC_Door_Open_Close.Play_SC_Door_Open_Close" _self)
    (bind _angle (Timeline|Timeline_0 Play)
      (:Update
        (Transformation|SetRelativeRotation (Variables|Default|GetClosetsDoorC_Door) (Math|Rotator|MakeRotator 0.0 0.0 _angle) false false)))
    (else
      (Variables|Default|SetOpen? false)
      (Class|AkGameplayStatics|PostEvent "/Game/WwiseAudio/Events/Hassan/Play_SC_Door_Open_Close.Play_SC_Door_Open_Close" _self)
      (Timeline|Timeline_0 Reverse))))

(fn ConstructionScript)
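; Interactive TV stand actor whose four cabinet doors swing open and closed as two independent pairs.
; An OpenDoor event takes the hit component and picks the matching pair, A/B or C/D.
; Each pair has its own open flag that plays or reverses a timeline, yawing the two doors by mirrored angles.
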(event EventOpenDoor
  (params (hitComponent :type Actor%20Component%20Object%20Reference))
  (if (or (== hitComponent (Variables|Default|GetTVStand_DoorB)) (== hitComponent (Variables|Default|GetTVStand_DoorA)))
    (if (not (Variables|Default|GetOpen?))
      (Variables|Default|SetOpen? true)
      (bind _angle (Timeline|Timeline_0 Play)
        (:Update
          (Transformation|SetRelativeRotation (Variables|Default|GetTVStand_DoorA) (Math|Rotator|MakeRotator 0.0 0.0 _angle) false false)
          (Transformation|SetRelativeRotation (Variables|Default|GetTVStand_DoorB) (Math|Rotator|MakeRotator 0.0 0.0 (* _angle -1.0)) false false)))
      (else
        (Variables|Default|SetOpen? false)
        (Timeline|Timeline_0 Reverse)))
    (elif (or (== hitComponent (Variables|Default|GetTVStand_DoorC)) (== hitComponent (Variables|Default|GetTVStand_DoorD)))
      (if (not (Variables|Default|GetDoublePorteGauche))
        (Variables|Default|SetDoublePorteGauche true)
        (bind _angle_2 (Timeline|Timeline_1 Play)
          (:Update
            (Transformation|SetRelativeRotation (Variables|Default|GetTVStand_DoorC) (Math|Rotator|MakeRotator 0.0 0.0 _angle_2) false false)
            (Transformation|SetRelativeRotation (Variables|Default|GetTVStand_DoorD) (Math|Rotator|MakeRotator 0.0 0.0 (* _angle_2 -1.0)) false false)))
        (else
          (Variables|Default|SetDoublePorteGauche false)
          (Timeline|Timeline_1 Reverse))))))

(fn ConstructionScript)
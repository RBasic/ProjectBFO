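; BP_Desk is an interactable desk actor with two drawers that slide open and closed.
; The OpenDoor event checks whether the hit component is the left or right drawer and toggles that drawer's open flag.
; Each drawer has its own timeline, played or reversed to animate its relative Y location, with a Wwise drawer sound posted on every toggle.
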(event EventOpenDoor
  (params (hitComponent :type Actor%20Component%20Object%20Reference))
  (bind _self self)
  (bind _self_2 self)
  (bind _desk_drawer_l (Variables|Default|GetDesk_Drawer_L))
  (bind _desk_drawer_r (Variables|Default|GetDesk_Drawer_R))
  (bind _relativelocation (Variables|/Script/Engine.SceneComponent|GetRelativeLocation _desk_drawer_l))
  (bind _relativelocation_2 (Variables|/Script/Engine.SceneComponent|GetRelativeLocation _desk_drawer_r))
  (if (== hitComponent (Variables|Default|GetDesk_Drawer_L))
    (if (not (Variables|Default|GetOpenDrawerL?))
      (Variables|Default|SetOpenDrawerL? true)
      (Class|AkGameplayStatics|PostEvent "/Game/WwiseAudio/Events/Hassan/Play_SC_Drawner.Play_SC_Drawner" _self_2)
      (bind _movement (Timeline|Timeline_0 Play)
        (:Update
          (Transformation|SetRelativeLocation _desk_drawer_l (Math|Vector|MakeVector (.x _relativelocation) _movement (.z _relativelocation)) false false)))
      (else
        (Variables|Default|SetOpenDrawerL? false)
        (Class|AkGameplayStatics|PostEvent "/Game/WwiseAudio/Events/Hassan/Play_SC_Drawner.Play_SC_Drawner" _self_2)
        (Timeline|Timeline_0 Reverse)))
    (elif (== hitComponent (Variables|Default|GetDesk_Drawer_R))
      (if (not (Variables|Default|GetOpenDrawerR?))
        (Variables|Default|SetOpenDrawerR? true)
        (Class|AkGameplayStatics|PostEvent "/Game/WwiseAudio/Events/Hassan/Play_SC_Drawner.Play_SC_Drawner" _self)
        (bind _movement_2 (Timeline|Timeline_1 Play)
          (:Update
            (Transformation|SetRelativeLocation _desk_drawer_r (Math|Vector|MakeVector (.x _relativelocation_2) _movement_2 (.z _relativelocation_2)) false false)))
        (else
          (Variables|Default|SetOpenDrawerR? false)
          (Class|AkGameplayStatics|PostEvent "/Game/WwiseAudio/Events/Hassan/Play_SC_Drawner.Play_SC_Drawner" _self)
          (Timeline|Timeline_1 Reverse))))))

(fn ConstructionScript)
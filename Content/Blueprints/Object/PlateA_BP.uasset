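; PlateA_BP is a plate object that plays a Wwise glass sound when its static mesh hits a surface.
; Impact sounds are enabled only after a short delay following BeginPlay.
; Hits pass through a DoOnce, then post Play_Glass at the impact location if the physical material is carpet, concrete, wood or stairs.
; The DoOnce resets only after a sound posts, so a hit on any other material leaves it closed.
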(event OnComponentHit(StaticMeshComponent)
  (params (HitComponent :type Primitive%20Component%20Object%20Reference) (OtherActor :type Actor%20Object%20Reference) (OtherComp :type Primitive%20Component%20Object%20Reference) (NormalImpulse :type Vector :default "0, 0, 0") (Hit :type Hit%20Result%20Structure%20%28by%20ref%29))
  (if (Variables|Default|GetCanMakeSound?)
    (Utilities|FlowControl|DoOnce false :!label _label
      (:Completed
        (if (Math|Boolean|ORBoolean (== (.physmat Hit) "/Game/PhysicalMat/PhysicMat_Carpet.PhysicMat_Carpet") (== (.physmat Hit) "/Game/PhysicalMat/PhysicMat_Concrete.PhysicMat_Concrete") (== (.physmat Hit) "/Game/PhysicalMat/PhysicMat_Wood.PhysicMat_Wood") (== (.physmat Hit) "/Game/PhysicalMat/PhysicMat_Stairs.PhysicMat_Stairs") (== (.physmat Hit) "/Game/PhysicalMat/PhysicMat_Wood.PhysicMat_Wood"))
          (Class|AkGameplayStatics|PostEventatLocation "/Game/WwiseAudio/Events/Alexis/Play_Glass.Play_Glass" (.location Hit) "0, 0, 0")
          (goto _label Reset))))))

(event EventBeginPlay
  (Utilities|FlowControl|Delay 5.0)
  (Variables|Default|SetCanMakeSound? true))

(fn ConstructionScript)
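; BP_Thief is a player-controlled thief character Blueprint that owns and drives the thief's HUD.
; SpawnWidget creates a HUD_Voleur widget for the owning player controller and adds it to that player's screen.
; The OpenInventory input calls the widget's Inventaire function, while Tick runs the parent's logic and pushes the Message variable into the HUD's message text every frame.
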(event Custom|SpawnWidget
  (bind _returnvalue (UserInterface|CreateWidget "/Game/HUD/HUD_Voleur.HUD_Voleur_C" (.AsPlayer%20Controller (Utilities|Casting|CastToPlayerController (Pawn|GetController)))))
  (bind _output_get (Variables|Default|SetHUD_Voleur _returnvalue))
  (UserInterface|Viewport|AddtoPlayerScreen _output_get))

(event EventTick
  (params (DeltaSeconds :type Float%20%28single-precision%29))
  (|CallParentFunction DeltaSeconds)
  (Rendering|Components|TextRender|SetText (Variables|/Game/HUD/HUD_Voleur.HUD_Voleur_C|GetMessage (Variables|Default|GetHUD_Voleur)) (Variables|Default|GetMessage)))

(event Input|ActionEvents|InputActionOpenInventory
  (params (Key :type Key%20Structure :default "None"))
  (:Pressed
    (Default|Inventaire (Variables|Default|GetHUD_Voleur))))

(fn ConstructionScript
  (|CallParentFunction))
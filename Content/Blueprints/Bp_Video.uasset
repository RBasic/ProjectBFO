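; Video screen actor that toggles playback of a media source on a plane mesh.
; On BeginPlay it assigns a material to the plane.
; Each Activate event flips the IsPlaying flag, either showing the plane and opening the Video source in the media player, or closing the player and hiding the plane.
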(event Custom|Activate
  (if (not (Variables|Default|GetIsPlaying))
    (Rendering|SetVisibility (Variables|Default|GetPlane) true false)
    (Media|MediaPlayer|OpenSource (Variables|Default|GetMediaplayer) "/Game/Sounds/Video.Video")
    (Variables|Default|SetIsPlaying true)
    (else
      (Media|MediaPlayer|Close (Variables|Default|GetMediaplayer) :!class /Script/MediaAssets.MediaPlayer)
      (Rendering|SetVisibility (Variables|Default|GetPlane) false false)
      (Variables|Default|SetIsPlaying false))))

(event EventBeginPlay
  (Rendering|Material|SetMaterial (Variables|Default|GetPlane) 0 (Variables|Default|GetNewVar_0)))

(fn ConstructionScript)